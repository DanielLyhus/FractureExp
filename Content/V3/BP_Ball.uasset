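; BP_Ball is a player-controlled physics ball that rolls via input torque in a slow-motion world.
; Hits on simulating bodies briefly spawn and trigger an FS_MasterField at the impact with camera shake; a polling timer also shakes the camera on landings.
; First move input creates a level-specific HUD and starts its clock timer.
; The ball also handles retry by level reload and a pause menu.
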(event Custom|CheckIfLanding
  (bind _returnvalue (Physics|GetPhysicsLinearVelocity (Variables|Default|GetSphere) "None"))
  (if (< (.z _returnvalue) -5e+01)
    (if (not (Variables|Default|GetFalling))
      (Variables|Default|SetFalling true))
    (elif (Variables|Default|GetFalling)
      (Variables|Default|SetFalling false)
      (Camera|PlayWorldCameraShake "/Game/CS_Base.CS_Base_C" (Transformation|GetWorldLocation (Variables|Default|GetSphere)) 2e+02 1e+03 1.0 true))))

(event Custom|E_Unpause
  (bind _returnvalue (Game|GetPlayerController 0))
  (Widget|RemovefromParent (stale Input|EnhancedActionEvents|EnhancedInputActionIA_Pause _returnvalue_2))
  (Game|SetGamePaused false)
  (Variables|/Script/Engine.PlayerController|SetbShowMouseCursor _returnvalue false)
  (Input|SetInputModeGameOnly _returnvalue false))

(event Custom|E_TimerD
  (bind _foundwidgets (Widget|GetAllWidgetsOfClass "/Game/UI/WBP_UID.WBP_UID_C" true))
  (for _array_element _foundwidgets
    (Default|UpdateClock _array_element)))

(event Custom|E_Timer
  (bind _foundwidgets (Widget|GetAllWidgetsOfClass "/Game/UI/WBP_UIC.WBP_UIC_C" true))
  (for _array_element _foundwidgets
    (Default|UpdateClock _array_element)))

(event Input|EnhancedActionEvents|EnhancedInputActionIA_Move
  (params (ActionValue :type Vector%202D%20Structure) (ElapsedSeconds :type Float%20%28double-precision%29) (TriggeredSeconds :type Float%20%28double-precision%29) (InputAction :type Input%20Action%20Object%20Reference :default "/Game/Input/Actions/IA_Move.IA_Move"))
  (bind _torquemultiplier (Variables|Default|GetTorqueMultiplier))
  (Utilities|FlowControl|Sequence
    (:then_0
      (Utilities|FlowControl|DoOnce false
        (:Completed
          (bind _returnvalue (Game|GetCurrentLevelName true))
          (if (Utilities|Enum|Equal(Enum) _returnvalue "MAP_02")
            (bind _returnvalue_2 (UserInterface|CreateWidget "/Game/UI/WBP_UID.WBP_UID_C"))
            (UserInterface|Viewport|AddtoViewport _returnvalue_2 0)
            (Utilities|Time|SetTimerbyEvent (delegate Custom|E_TimerD) 0.4 true)
            (else
              (bind _returnvalue_3 (UserInterface|CreateWidget "/Game/UI/WBP_UIC.WBP_UIC_C" (Game|GetPlayerController 0)))
              (UserInterface|Viewport|AddtoViewport _returnvalue_3 0)
              (Utilities|Time|SetTimerbyEvent (delegate Custom|E_Timer) 0.4 true))))))
    (:then_1
      (Class|PrimitiveComponent|AddTorqueinDegrees (Variables|Default|GetSphere) (Math|Vector|MakeVector (* (* (.x ActionValue) -1.0) _torquemultiplier) (* (.y ActionValue) _torquemultiplier) 0.0) "None" true))))

(event Input|EnhancedActionEvents|EnhancedInputActionIA_Pause
  (params (ActionValue :type Boolean) (ElapsedSeconds :type Float%20%28double-precision%29) (TriggeredSeconds :type Float%20%28double-precision%29) (InputAction :type Input%20Action%20Object%20Reference :default "/Game/Input/Actions/IA_Pause.IA_Pause"))
  (bind _returnvalue (Game|GetPlayerController 0))
  (:Completed
    (if (Game|IsGamePaused)
      (Widget|RemovefromParent (stale _returnvalue_2))
      (Game|SetGamePaused false)
      (Variables|/Script/Engine.PlayerController|SetbShowMouseCursor _returnvalue false)
      (Input|SetInputModeGameOnly _returnvalue false)
      (else
        (bind _returnvalue_2 (UserInterface|CreateWidget "/Game/UI/WBP_Pause.WBP_Pause_C" _returnvalue))
        (UserInterface|Viewport|AddtoViewport _returnvalue_2 0)
        (Game|SetGamePaused true)
        (Variables|/Script/Engine.PlayerController|SetbShowMouseCursor _returnvalue true)
        (Input|SetInputModeGameandUI _returnvalue _returnvalue_2 "DoNotLock" true false)))))

(event Input|EnhancedActionEvents|EnhancedInputActionIA_Retry
  (params (ActionValue :type Boolean) (ElapsedSeconds :type Float%20%28double-precision%29) (TriggeredSeconds :type Float%20%28double-precision%29) (InputAction :type Input%20Action%20Object%20Reference :default "/Game/Input/Actions/IA_Retry.IA_Retry"))
  (:Completed
    (bind _returnvalue (UserInterface|CreateWidget "/Game/UI/WBP_Retrying.WBP_Retrying_C"))
    (UserInterface|Viewport|AddtoViewport _returnvalue 0)
    (bind _returnvalue_2 (Game|GetCurrentLevelName true))
    (Game|OpenLevel(byName) (Utilities|String|StringToName _returnvalue_2))))

(event Collision|EventHit
  (params (MyComp :type Primitive%20Component%20Object%20Reference) (Other :type Actor%20Object%20Reference) (OtherComp :type Primitive%20Component%20Object%20Reference) (bSelfMoved :type Boolean) (HitLocation :type Vector :default "0, 0, 0") (HitNormal :type Vector :default "0, 0, 0") (NormalImpulse :type Vector :default "0, 0, 0") (Hit :type Hit%20Result%20Structure%20%28by%20ref%29))
  (if (Physics|IsSimulatingPhysics OtherComp "None")
    (Utilities|FlowControl|DoOnce false :!label _label
      (:Completed
        (bind _returnvalue (Game|SpawnActorfromClass "/Engine/EditorResources/FieldNodes/FS_MasterField.FS_MasterField_C" (Math|Transform|MakeTransform HitLocation) "Undefined" "MultiplyWithRoot" 0 0))
        (Variables|/Engine/EditorResources/FieldNodes/FS_MasterField.FS_MasterField_C|SetActivationType _returnvalue "NewEnumerator4")
        (Default|CETrigger _returnvalue)
        (Camera|PlayWorldCameraShake "/Game/CS_Base.CS_Base_C" HitLocation 2e+02 2e+03 1.0 true)
        (Utilities|FlowControl|Delay 0.05)
        (Actor|DestroyActor _returnvalue)
        (goto _label Reset)))))

(event EventBeginPlay
  (Utilities|Time|SetGlobalTimeDilation 0.4)
  (Class|PrimitiveComponent|SetPhysicsMaxAngularVelocityinDegrees (Variables|Default|GetSphere) 1e+03 false "None")
  (Utilities|Time|SetTimerbyEvent (delegate Custom|CheckIfLanding) 0.01 true true))

(fn ConstructionScript)